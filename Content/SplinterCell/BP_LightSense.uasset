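; BP_LightSense is a light sensor in the SplinterCell folder that measures a light value from the RT_LightSense render target.
; A looping timer started on BeginPlay samples three fixed pixels in a triangle every 0.05 seconds and averages their raw red channels into LightValue.
; The BPI_LightValue interface function returns that cached value, so callers do not trigger a render target read themselves.
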(event `self.ReceiveBeginPlay`
  (bind _returnvalue (`KismetSystemLibrary.K2_SetTimerDelegate` (delegate `Read`) 0.05 true))
  (set `self.TimerRead` _returnvalue))

(event `Read`
  (bind _returnvalue (`KismetRenderingLibrary.ReadRenderTargetRawPixel` "/Game/SplinterCell/RT_LightSense.RT_LightSense" 128 55))
  (bind _returnvalue_2 (`KismetRenderingLibrary.ReadRenderTargetRawPixel` "/Game/SplinterCell/RT_LightSense.RT_LightSense" 55 180))
  (bind _returnvalue_3 (`KismetRenderingLibrary.ReadRenderTargetRawPixel` "/Game/SplinterCell/RT_LightSense.RT_LightSense" 192 180))
  (set `self.LightValue` (/ (+ (break `LinearColor` _returnvalue) (break `LinearColor` _returnvalue_2) (break `LinearColor` _returnvalue_3)) 3.0)))

(fn `BPI_LightValue`
  (returns (LightValue :type "Float (double-precision)"))
  (return (`self.LightValue`)))

(fn `UserConstructionScript`)