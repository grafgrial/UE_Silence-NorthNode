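; AC_StorePoint is a purchasable store location that shows its price on floating text turned toward the player each tick.
; Sphere overlap with a BPI_Player actor enables input and opens a gate for the E key.
; E queries the Manager through interface calls: if already sold it only prints a store-open debug message, otherwise it sends a purchase or insufficient-money message.
; Leaving the sphere disables input, closes the gate and clears that warning.
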(event `self.ReceiveBeginPlay`
  (`TextRenderComponent.K2_SetText` (`self.TextRender`) (`KismetTextLibrary.Conv_DoubleToText` (`self.Price`) "HalfToEven")))

(event `self.ReceiveTick`
  (params (DeltaSeconds :type "Float (single-precision)"))
  (bind _returnvalue (`GameplayStatics.GetPlayerCharacter` 0))
  (`/Engine/EditorBlueprintResources/StandardMacros.IsValid` _returnvalue
    (:`Is Valid`
      (`SceneComponent.K2_SetWorldRotation` (`self.TextRender`) (`KismetMathLibrary.FindLookAtRotation` (`self.K2_GetActorLocation`) (`self.K2_GetActorLocation` _returnvalue)) false false))))

(event `Key|E`
  (params (Key :type "Key Structure"))
  (:`Pressed`
    (`/Engine/EditorBlueprintResources/StandardMacros.Gate` true :!label _label
      (:`Exit`
        (bind _manager (`self.Manager`)
          (:`then`
            (bind (_sell _money) (message `/Game/Tow/BPI_Manager.BPI_Manager_IsSell?` _manager))
            (if _sell
              (`KismetSystemLibrary.PrintString` "TRUE Магазин открыт. Создаем виджет")
              (elif (>= _money (`self.Price`))
                (`KismetSystemLibrary.PrintString` "FALSE больше денег")
                (message `/Game/Tow/BPI_Manager.BPI_Manager_Sell` (`self.Manager`) (`self.Price`) (`self.Name`))
                (else
                  (`KismetSystemLibrary.PrintString` "FALSE Нет денег")
                  (message `/Game/Tow/BPI_Manager.BPI_Manager_WidgetNoSell` (`self.Manager`) true)))))
          (:`else`))))))

(event `self.Sphere.OnComponentBeginOverlap`
  (params (OverlappedComponent :type "PrimitiveComponent Object Reference") (OtherActor :type "Actor Object Reference") (OtherComp :type "PrimitiveComponent Object Reference") (OtherBodyIndex :type Integer) (bFromSweep :type Boolean) (SweepResult :type "HitResult Structure (by ref)"))
  (if (`KismetSystemLibrary.DoesImplementInterface` OtherActor "/Game/AGAME/Base/Interface/BPI_PLayer.BPI_Player_C")
    (`self.EnableInput` (`GameplayStatics.GetPlayerController` 0))
    (goto _label :!via `Open`)))

(event `self.Sphere.OnComponentEndOverlap`
  (params (OverlappedComponent :type "PrimitiveComponent Object Reference") (OtherActor :type "Actor Object Reference") (OtherComp :type "PrimitiveComponent Object Reference") (OtherBodyIndex :type Integer))
  (if (`KismetSystemLibrary.DoesImplementInterface` OtherActor "/Game/AGAME/Base/Interface/BPI_PLayer.BPI_Player_C")
    (`self.DisableInput` (`GameplayStatics.GetPlayerController` 0))
    (bind _manager (`self.Manager`)
      (:`then`
        (message `/Game/Tow/BPI_Manager.BPI_Manager_WidgetNoSell` _manager false)
        (goto _label :!via `Close`))
      (:`else`
        (goto _label :!via `Close`)))))

(fn `UserConstructionScript`)