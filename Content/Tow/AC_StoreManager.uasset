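; AC_StoreManager is a store manager actor that owns the player's money and spawns AC_StorePoint purchase spots at preset offsets from itself.
; BeginPlay creates the WB_Money HUD, registers one named item and spawns the first point with a reference back to the manager.
; Interface sale events remove the item, deduct its price, refresh the HUD and spawn the next point if named items remain.
; Other interface calls toggle a no-sale border and report sale state and money.
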(event `self.ReceiveBeginPlay`
  (bind _storecell_0 (`self.StoreCell_0`))
  (bind _returnvalue (`|CreateWidget` "/Game/Tow/Widget/WB_Money.WB_Money_C"))
  (bind _output_get (set `self.Widget` _returnvalue))
  (`UserWidget.AddToViewport` _output_get 0)
  (`BlueprintMapLibrary.Map_Add` _storecell_0 "Name1" true)
  (`|SpawnActorFromClass` "/Game/Tow/AC_StorePoint.AC_StorePoint_C" (`KismetMathLibrary.MakeTransform` (+ (`self.K2_GetActorLocation`) (`|GetArrayItem` (`self.StorePoint`) (`self.NewVar_0`)))) "Undefined" "OverrideRootScale" null self (`.ReturnValue` (`BlueprintMapLibrary.Map_Find` _storecell_0 "Name1")) 100.0 "Name1" null)
  (`/Game/Tow/Widget/WB_Money.DISP_Update` (`self.Widget`) (`self.Money`)))

(event `E_Spawn`
  (bind _newvar_0 (`self.NewVar_0`))
  (set `self.NewVar_0` (+ (`self.NewVar_0`) 1))
  (`BlueprintMapLibrary.Map_Add` (`self.StoreCell`) _newvar_0)
  (bind _keys (`BlueprintMapLibrary.Map_Keys` (`self.StoreCell_0`)))
  (if (> (`KismetArrayLibrary.Array_Length` _keys) 0)
    (`|SpawnActorFromClass` "/Game/Tow/AC_StorePoint.AC_StorePoint_C" (`KismetMathLibrary.MakeTransform` (+ (`self.K2_GetActorLocation`) (`|GetArrayItem` (`self.StorePoint`) _newvar_0))) "Undefined" "OverrideRootScale" null self false (`self.Price`) (`|GetArrayItem` _keys) null)
    (`/Game/Tow/Widget/WB_Money.DISP_Update` (`self.Widget`) (`self.Money`))))

(event `/Game/Tow/BPI_Manager.BPI_Manager_Sell`
  (params (Price :type "Float (single-precision)") (Name :type Name))
  (if (`.ReturnValue` (`BlueprintMapLibrary.Map_Find` (`self.StoreCell_0`) Name))
    (bind _returnvalue (`BlueprintMapLibrary.Map_Remove` (`self.StoreCell_0`) Name))
    (if _returnvalue
      (bind _output_get (set `self.Money` (- (`self.Money`) Price)))
      (`/Game/Tow/Widget/WB_Money.DISP_Update` (`self.Widget`) _output_get)
      (`self.E_Spawn`))))

(event `/Game/Tow/BPI_Manager.BPI_Manager_WidgetNoSell`
  (params (NewParam :type Boolean))
  (bind _border_87 (`/Game/Tow/Widget/WB_Money.Border_87` (`self.Widget`)))
  (if NewParam
    (`Widget.SetVisibility` _border_87 "Visible")
    (else
      (`Widget.SetVisibility` _border_87 "Collapsed"))))

(fn `BPI_Manager_IsSell?`
  (returns (Sell :type Boolean) (Money :type "Float (double-precision)"))
  (return (`.ReturnValue` (`BlueprintMapLibrary.Map_Find` (`self.StoreCell`))) (`self.Money`)))

(fn `RefreshMoney`
  (`/Game/Tow/Widget/WB_Money.DISP_Update` (`self.Widget`) (`self.Money`)))

(fn `UserConstructionScript`)