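; Slot machine actor for the casino: interacting with its lever plays a sound, animates the pull and starts a one-time spin.
; ActionHear rolls a random six-position result and target angle per wheel, then sets a timer that assigns Deceleration.
; Tick sets each wheel's roll from speed times delta, then overwrites that speed with Deceleration times delta.
; Stopping is unfinished: target angles go unused, IsSpinning never resets and Stop2 is empty.
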(event `/Game/AGAME/Base/Interface/BPI_Interaction.BPI_Iteraction`
  (params (Pawn :type "Pawn Object Reference") (Component :type "PrimitiveComponent Object Reference"))
  (if (== Component (`self.slot_Cylinder`))
    (`GameplayStatics.PlaySoundAtLocation` (`self.Sound`) (`self.K2_GetActorLocation`) (struct) 1.0 1.0 0.0 null null null)
    (`self.Ruchka`)
    (`self.ActionHear`)))

(event `Ruchka`
  (if (not (`self.IsTriggerRuchka`))
    (bind (_direction _alpha) (`Timeline|ruchka_timeline` :!via `PlayFromStart`)
      (:`Update`
        (`SceneComponent.K2_SetRelativeRotation` (`self.slot_Cylinder`) (`KismetMathLibrary.MakeRotator` (`KismetMathLibrary.Lerp` 0.0 -30.0 _alpha)) false false)))))

(event `self.ReceiveBeginPlay`
  (set `self.WheelArray` (`|MakeArray` (`self.Wheel_3`) (`self.Wheel_2`) (`self.Wheel_1`))))

(event `self.ReceiveTick`
  (params (DeltaSeconds :type "Float (single-precision)"))
  (if (`self.IsSpinning`)
    (for _index (range 3)
      (if (> (`|GetArrayItem` (`self.CurrentSpinSpeed`) _index) 0.0)
        (bind _returnvalue (* (`|GetArrayItem` (`self.CurrentSpinSpeed`) _index) (`GameplayStatics.GetWorldDeltaSeconds`)))
        (`KismetSystemLibrary.PrintString` (`KismetStringLibrary.Conv_DoubleToString` _returnvalue))
        (`SceneComponent.K2_SetRelativeRotation` (`|GetArrayItem` (`self.WheelArray`) _index) (`KismetMathLibrary.MakeRotator` _returnvalue) false false)
        (`KismetArrayLibrary.Array_Set` (`self.CurrentSpinSpeed`) _index (* (`self.Deceleration`) (`GameplayStatics.GetWorldDeltaSeconds`)))))))

(event `ActionHear`
  (if (not (`self.IsSpinning`))
    (for _index (range 3)
      (`KismetArrayLibrary.Array_Add` (`self.CurrentSpinSpeed`) (`self.SpinSpeed`))
      (`KismetArrayLibrary.Array_Add` (`self.Results`) (`KismetMathLibrary.RandomIntegerInRange` 0 5))
      (`KismetArrayLibrary.Array_Add` (`self.TargetStopAngles`) (+ (`KismetMathLibrary.Conv_IntToDouble` (* (`|GetArrayItem` (`self.Results`) _index) 60)) (* 360.0 (`KismetMathLibrary.RandomFloatInRange` 4.0 6.0)))))
    (`KismetSystemLibrary.K2_SetTimerDelegate` (delegate `Stop1`) 2.0)
    (set `self.IsSpinning` true)))

(event `Stop1`
  (set `self.Deceleration` 500.0))

(event `Stop2`)

(fn `UserConstructionScript`)