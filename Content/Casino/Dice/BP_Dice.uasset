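; BP_Dice is a physics-driven casino die that rolls itself on BeginPlay and prints the face it lands on.
; StartRoll applies a mass-scaled random impulse, kept upward, plus random torque, then opens a Tick gate after a short delay.
; Once velocity drops near zero, ReadValue finds the highest mesh socket, whose name is looked up in SideValues and printed once.
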(event `self.ReceiveBeginPlay`
  (`self.StartRoll` 800.0))

(event `self.ReceiveTick`
  (params (DeltaSeconds :type "Float (single-precision)"))
  (`/Engine/EditorBlueprintResources/StandardMacros.Gate` true :!label _label
    (:`Exit`
      (if (<= (`KismetMathLibrary.VSize` (`self.GetVelocity`)) 5.0)
        (`/Engine/EditorBlueprintResources/StandardMacros.DoOnce` false
          (:`Completed`
            (bind _l_highestname1 (`self.ReadValue`))
            (`KismetSystemLibrary.PrintString` (`KismetStringLibrary.Conv_IntToString` (`BlueprintMapLibrary.Map_Find` (`self.SideValues`) _l_highestname1)))))))))

(event `Rolled`
  (`KismetSystemLibrary.Delay` 0.2)
  (goto _label :!via `Open`))

(fn `ReadValue`
  (returns (L_HighestName1 :type Name))
  (locals (L_HighestValue :type "Float (double-precision)") (L_HighestName :type Name))
  (for _array_element (`SceneComponent.GetAllSocketNames` (`self.Dice1`))
    (bind (_returnvalue_x _returnvalue_y _returnvalue_z) (`KismetMathLibrary.BreakVector` (`SceneComponent.GetSocketLocation` (`self.Dice1`) _array_element)))
    (if (> _returnvalue_z (`local.L_HighestValue`))
      (set `local.L_HighestValue` _returnvalue_z)
      (set `local.L_HighestName` _array_element)))
  (return (`local.L_HighestName`)))

(fn `StartRoll`
  (params (B :type "Float (double-precision)"))
  (bind _dice1 (`self.Dice1`))
  (bind (_returnvalue_x _returnvalue_y _returnvalue_z) (`KismetMathLibrary.BreakVector` (* (* (`KismetMathLibrary.RandomUnitVector`) (`PrimitiveComponent.GetMass` (`self.Dice1`))) B)))
  (`PrimitiveComponent.AddImpulse` _dice1 (`KismetMathLibrary.MakeVector` _returnvalue_x _returnvalue_y (`KismetMathLibrary.Abs` _returnvalue_z)) "None" false)
  (`PrimitiveComponent.AddTorqueInDegrees` _dice1 (* (* (* (`KismetMathLibrary.RandomUnitVector`) (`PrimitiveComponent.GetMass` (`self.Dice1`))) B) 300000.0) "None" false)
  (`self.Rolled`))

(fn `UserConstructionScript`)