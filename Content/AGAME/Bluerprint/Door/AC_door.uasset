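; AC_door is an interactable door that swings open and shut, optionally gated by a key.
; Interacting with its Cube either starts the swing or, if Iskey is set, passes the door and Key to the pawn's first BPI_KeyDoor component.
; BPIKeyOut enters the same DoOnce, bypassing the key check.
; A timeline lerps the Scene rotation, then flips DoorClosed and resets the DoOnce, which blocks retriggering mid-swing.
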(event `/Game/AGAME/Base/Interface/BPI_Interaction.BPI_Iteraction`
  (params (Pawn :type "Pawn Object Reference") (Component :type "PrimitiveComponent Object Reference"))
  (if (== Component (`self.Cube`))
    (if (`self.Iskey?`)
      (message `/Game/AGAME/Bluerprint/Door/BPI_KeyDoor.BPI_KeyInput` (`|GetArrayItem` (`self.GetComponentsByInterface` Pawn "/Game/AGAME/Bluerprint/Door/BPI_KeyDoor.BPI_KeyDoor_C")) self (`self.Key`))
      (else
        (`/Engine/EditorBlueprintResources/StandardMacros.DoOnce` false :!label _label
          (:`Completed`
            (bind (_direction _newtrack_0) (`Timeline|Timeline_0` :!via `PlayFromStart`)
              (:`Update`
                (`SceneComponent.K2_SetRelativeRotation` (`self.Scene`) (`KismetMathLibrary.RLerp` (select `bool` (`self.DoorClosed?`) :`false` (struct :`Yaw` 80.0) :!type "Rotator Structure") (select `bool` (not (`self.DoorClosed?`)) :`false` (struct :`Yaw` 80.0) :!type "Rotator Structure") _newtrack_0) false false))
              (:`Finished`
                (if (`self.DoorClosed?`)
                  (set `self.DoorClosed?` false)
                  (else
                    (set `self.DoorClosed?` true)))
                (`self.E_Reset`)))))))))

(event `/Game/AGAME/Bluerprint/Door/BPI_KeyOut.BPI_KeyOut`
  (goto _label))

(event `E_Reset`
  (goto _label :!via `Reset`))

(fn `UserConstructionScript`)