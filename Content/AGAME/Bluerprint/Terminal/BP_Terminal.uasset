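; BP_Terminal is an interactive terminal actor that takes over the player's view when the player character enters its Box trigger.
; On overlap it blends the camera to itself, enables its own input, shows the mouse cursor and activates its WidgetInteraction component.
; Right mouse press and release are forwarded to that component as left-mouse pointer clicks.
; The graph has no exit logic to restore the view or input.
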(event `self.Box.OnComponentBeginOverlap`
  (params (OverlappedComponent :type "PrimitiveComponent Object Reference") (OtherActor :type "Actor Object Reference") (OtherComp :type "PrimitiveComponent Object Reference") (OtherBodyIndex :type Integer) (bFromSweep :type Boolean) (SweepResult :type "HitResult Structure (by ref)"))
  (bind _returnvalue (`GameplayStatics.GetPlayerController` 0))
  (if (== OtherActor (`GameplayStatics.GetPlayerCharacter` 0))
    (`PlayerController.SetViewTargetWithBlend` (`GameplayStatics.GetPlayerController` 0) self 0.6 "VTBlend_Cubic" 0.0 false)
    (`self.EnableInput` _returnvalue)
    (set `PlayerController.bShowMouseCursor` true _returnvalue)
    (`ActorComponent.Activate` (`self.WidgetInteraction`) false)))

(event `Key|RightMouseButton`
  (params (Key :type "Key Structure"))
  (bind _widgetinteraction (`self.WidgetInteraction`))
  (:`Pressed`
    (`WidgetInteractionComponent.PressPointerKey` _widgetinteraction "LeftMouseButton"))
  (:`Released`
    (`WidgetInteractionComponent.ReleasePointerKey` _widgetinteraction "LeftMouseButton")))

(fn `UserConstructionScript`)