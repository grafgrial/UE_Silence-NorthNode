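; BP_BaseGUN is a base gun actor that can be looked at and interacted with in the world.
; Its construction script pulls the static mesh and name from the PDA data asset's struct, so the asset drives each gun's appearance and label.
; The look-at interface returns that name as text, and interacting with the mesh only destroys the actor, with no item handed over here.
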(event `/Game/AGAME/Base/Interface/BPI_Interaction.BPI_Iteraction`
  (params (Pawn :type "Pawn Object Reference") (Component :type "PrimitiveComponent Object Reference"))
  (if (== Component (`self.Mesh`))
    (`self.K2_DestroyActor`)))

(fn `BPI_LookAt`
  (returns (Message :type Text))
  (return (`KismetTextLibrary.Conv_NameToText` (`self.Name`))))

(fn `UserConstructionScript`
  (bind (_type _mesh _magazin _name) (break `/Game/AGAME/Bluerprint/Gun/STR_Gun` (`/Game/AGAME/Bluerprint/Gun/PDA_Gun.STR` (`self.PDA`))))
  (`StaticMeshComponent.SetStaticMesh` (`self.Mesh`) _mesh)
  (set `self.Name` _name))