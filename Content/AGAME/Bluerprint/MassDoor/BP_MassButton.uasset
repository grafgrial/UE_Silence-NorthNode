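; BP_MassButton is a pressure plate that totals the mass of overlapping actors and reports it to a linked BP_ObjectDoor.
; Box overlaps add or remove each actor's mass in a map, keeping the total clamped between zero and TargetMass.
; When the mass fraction changes, it calls the door's DISPMas with the current mass and enables Tick.
; Tick interpolates the Cube's height toward that fraction, then disables itself upon reaching it.
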(event `self.Box.OnComponentBeginOverlap`
  (params (OverlappedComponent :type "PrimitiveComponent Object Reference") (OtherActor :type "Actor Object Reference") (OtherComp :type "PrimitiveComponent Object Reference") (OtherBodyIndex :type Integer) (bFromSweep :type Boolean) (SweepResult :type "HitResult Structure (by ref)"))
  (`self.CountTesting` OtherActor OtherComp true)
  (`self.UpdateStats` :!label _label))

(event `self.Box.OnComponentEndOverlap`
  (params (OverlappedComponent :type "PrimitiveComponent Object Reference") (OtherActor :type "Actor Object Reference") (OtherComp :type "PrimitiveComponent Object Reference") (OtherBodyIndex :type Integer))
  (`self.CountTesting` OtherActor OtherComp)
  (goto _label))

(event `Testing`
  (for _array_element (`self.Other Comp`)
    (bind _output_get (set `self.CurrentMass` (+ (`self.CurrentMass`) (`PrimitiveComponent.GetMass` _array_element))))
    (`KismetSystemLibrary.PrintString` (`KismetStringLibrary.Conv_DoubleToString` _output_get) true true (struct :`R` 1.0 :`B` 0.092422 :`A` 1.0) 10.0)))

(event `self.ReceiveTick`
  (params (DeltaSeconds :type "Float (single-precision)"))
  (if (== (`self.Location Z`) (`self.CurrentPersent`))
    (`self.SetActorTickEnabled` false)
    (else
      (set `self.Location Z` (`KismetMathLibrary.FInterpTo` (`self.Location Z`) (`self.CurrentPersent`) (`GameplayStatics.GetWorldDeltaSeconds`) 10.0))
      (set `self.New Location` (`KismetMathLibrary.MakeVector` 0.0 0.0 (`KismetMathLibrary.Lerp` 5.0 -7.0 (`self.Location Z`))))
      (`SceneComponent.K2_SetRelativeLocation` (`self.Cube`) (`self.New Location`) false false))))

(fn `CountTesting`
  (params (Actor :type "Actor Object Reference") (Primitive :type "PrimitiveComponent Object Reference") (bPlus :type Boolean))
  (bind _value (`BlueprintMapLibrary.Map_Find` (`self.ActorMass`) (`local.Actor`)))
  (if bPlus
    (`BlueprintMapLibrary.Map_Add` (`self.ActorMass`) (`local.Actor`) (`PrimitiveComponent.GetMass` (`local.Primitive`))))
  (if (<= (`BlueprintMapLibrary.Map_Length` (`self.ActorMass`)) 0)
    (set `self.CurrentMass` 0.0)
    (else
      (set `self.CurrentMass` (`KismetMathLibrary.FClamp` (+ (`self.CurrentMass`) (select `bool` bPlus :`false` (* _value -1.0) :`true` _value)) 0.0 (`self.TargetMass`)))))
  (if (not bPlus)
    (`BlueprintMapLibrary.Map_Remove` (`self.ActorMass`) (`local.Actor`))))

(fn `UpdateStats`
  (bind _returnvalue (`KismetMathLibrary.FClamp` (/ (`self.CurrentMass`) (`self.TargetMass`))))
  (if (not (== (`self.CurrentPersent`) _returnvalue))
    (set `self.CurrentPersent` _returnvalue)
    (`self.SetActorTickEnabled` true)
    (bind _object (`self.Object`)
      (:`then`
        (bind _asbp_object_door (cast `/Game/AGAME/Bluerprint/MassDoor/BP_ObjectDoor` _object))
        (`/Game/AGAME/Bluerprint/MassDoor/BP_ObjectDoor.DISP_Mas` _asbp_object_door (`self.CurrentMass`)))
      (:`else`))))

(fn `UserConstructionScript`)