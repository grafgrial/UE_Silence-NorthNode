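; BP_Fonar is a spotlight lamp actor that a pawn can interact with, apparently as a pickup.
; FonarOn fades the SpotLight intensity in through a timeline and reverses it to switch off, while the construction script sets the initial state from IsOn.
; Interacting with the StaticMesh sends the actor to the pawn through an attach message, then destroys it.
; The IsOn toggle logic is left unconnected.
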(event `self.ReceiveBeginPlay`)

(event `FonarOn`
  (params (`bIsOn?` :type Boolean))
  (if `bIsOn?`
    (bind (_direction _alpha) (`Timeline|FonarOn_timeline` :!via `PlayFromStart` :!label _label)
      (:`Update`
        (`LightComponent.SetIntensity` (`self.SpotLight`) (`KismetMathLibrary.Lerp` 0.0 (`self.Intensity`) _alpha))))
    (else
      (goto _label :!via `Reverse`))))

(event `/Game/AGAME/Base/Interface/BPI_Interaction.BPI_Iteraction`
  (params (Pawn :type "Pawn Object Reference") (Component :type "PrimitiveComponent Object Reference"))
  (if (== Component (`self.StaticMesh`))
    (message `/Game/AGAME/Base/Interface/BPI_PLayer.BPI_AttachActor` Pawn self)
    (`self.K2_DestroyActor`)))

(fn `UserConstructionScript`
  (if (`self.bIsOn?`)
    (set `self.bIsOn?` true)
    (`LightComponent.SetIntensity` (`self.SpotLight`) (`self.Intensity`))
    (`TimelineComponent.SetNewTime` (`self.FonarOn_timeline`) 1.35)
    (else
      (set `self.bIsOn?` false)
      (`LightComponent.SetIntensity` (`self.SpotLight`) 0.0))))