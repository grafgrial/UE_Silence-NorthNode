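; AC_Letter is an interactable letter actor whose texture, name and text come from a PDALetter data asset.
; The construction script creates a dynamic MM_Letter material instance, sets its Letter texture, applies it to LetterMesh and copies the letter data into variables.
; It implements interaction and look-at interface hooks, but the LetterMesh interaction branch does nothing and look-at returns an empty string.
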(event `/Game/AGAME/Base/Interface/BPI_Interaction.BPI_Iteraction`
  (params (Pawn :type "Pawn Object Reference") (Component :type "PrimitiveComponent Object Reference"))
  (if (== Component (`self.Letter_mesh`))
    _))

(fn `BPI_LookAt`
  (returns (Message :type Text))
  (return ""))

(fn `UserConstructionScript`
  (bind (_texture _name _text) (break `/Game/AGAME/Bluerprint/Letter/STR_Letter` (`/Game/AGAME/Bluerprint/Letter/PDA_Letter.STR_Letter` (`self.PDA_letter`))))
  (bind _returnvalue (`KismetMaterialLibrary.CreateDynamicMaterialInstance` "/Game/AGAME/Bluerprint/Letter/MM_Letter.MM_Letter"))
  (bind _output_get (set `self.Mat_Instance` _returnvalue))
  (`MaterialInstanceDynamic.SetTextureParameterValue` _output_get "Letter" _texture)
  (`PrimitiveComponent.SetMaterial` (`self.Letter_mesh`) 0 (`self.Mat_Instance`))
  (set `self.Texture` _texture)
  (set `self.Name` _name)
  (set `self.Text` _text))