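; AC_TriggerHorror is a configurable one-shot jump scare with two trigger volumes that respond only to the local player once IsLoaded is set.
; The Sphere overlap plays a 2D sound and removes itself, while the Box overlap starts the scare with a montage and screamer sound.
; A timeline slides the skeletal mesh between actor-relative start and stop offsets, then the actor destroys itself.
; The construction script applies the mesh, start position and timeline play rate.
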(event `self.Sphere.OnComponentBeginOverlap`
  (params (OverlappedComponent :type "PrimitiveComponent Object Reference") (OtherActor :type "Actor Object Reference") (OtherComp :type "PrimitiveComponent Object Reference") (OtherBodyIndex :type Integer) (bFromSweep :type Boolean) (SweepResult :type "HitResult Structure (by ref)"))
  (if (and (`self.IsLoaded?`) (== OtherActor (`GameplayStatics.GetPlayerCharacter` 0)))
    (`/Engine/EditorBlueprintResources/StandardMacros.DoOnce` false
      (:`Completed`
        (`GameplayStatics.SpawnSound2D` (`self.Sound`) 1.0 1.0 0.0 null)
        (`ActorComponent.K2_DestroyComponent` (`self.Sphere`))))))

(event `self.Box.OnComponentBeginOverlap`
  (params (OverlappedComponent :type "PrimitiveComponent Object Reference") (OtherActor :type "Actor Object Reference") (OtherComp :type "PrimitiveComponent Object Reference") (OtherBodyIndex :type Integer) (bFromSweep :type Boolean) (SweepResult :type "HitResult Structure (by ref)"))
  (if (and (`self.IsLoaded?`) (== OtherActor (`GameplayStatics.GetPlayerCharacter` 0)))
    (`/Engine/EditorBlueprintResources/StandardMacros.DoOnce` false
      (:`Completed`
        (`self.Run`)))))

(event `Run`
  (`|PlayMontage` (`self.SkeletalMesh`) (`self.Animation`)
    (:`then`
      (`GameplayStatics.SpawnSound2D` (`self.Sound_Skrimmer`) 1.0 1.0 0.0 null)
      (bind (_direction _newtrack_0) (`Timeline|Timeline_Run` :!via `PlayFromStart`)
        (:`Update`
          (`SceneComponent.K2_SetWorldLocation` (`self.SkeletalMesh`) (`KismetMathLibrary.VLerp` (+ (`self.K2_GetActorLocation`) (`self.PositionStart`)) (+ (`self.K2_GetActorLocation`) (`self.PositionStop`)) _newtrack_0) false false))
        (:`Finished`
          (`KismetSystemLibrary.Delay` 1.0)
          (`self.K2_DestroyActor`))))))

(fn `UserConstructionScript`
  (bind _skeletalmesh (`self.SkeletalMesh`))
  (bind _output_get (set `self.Time` (`self.Time`)))
  (`TimelineComponent.SetPlayRate` (`self.Timeline_Run`) _output_get)
  (`SkinnedMeshComponent.SetSkinnedAssetAndUpdate` _skeletalmesh (`self.MeshSkeletal`) true)
  (`SceneComponent.K2_SetWorldLocation` _skeletalmesh (+ (`self.K2_GetActorLocation`) (`self.PositionStart`)) false false))