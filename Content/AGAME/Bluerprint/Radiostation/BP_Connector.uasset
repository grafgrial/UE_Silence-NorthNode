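; BP_Connector is a colored, clickable connector cube for the radio station, tagged as left or right side.
; SpawnCon stores color and side, then drives the cube's R and G material parameters from remapped color bytes; blue goes to a parameter named "None".
; Clicking the cube passes the connector to the radio station's HandleConnectorClicked, but only when IsConnected is true.
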(event `SpawnCon`
  (params (Color :type "Color Structure") (bIsLeftSide :type Boolean))
  (set `self.Color` Color)
  (`MeshComponent.SetScalarParameterValueOnMaterials` (`self.Cube`) "R" (`KismetMathLibrary.MapRangeClamped` (`KismetMathLibrary.Conv_ByteToDouble` (`.R` (break `Color` (`self.Color`)))) 0.0 255.0 0.0 1.0))
  (`MeshComponent.SetScalarParameterValueOnMaterials` (`self.Cube`) "G" (`KismetMathLibrary.MapRangeClamped` (`KismetMathLibrary.Conv_ByteToDouble` (`.G` (break `Color` (`self.Color`)))) 0.0 255.0 0.0 1.0))
  (`MeshComponent.SetScalarParameterValueOnMaterials` (`self.Cube`) "None" (`KismetMathLibrary.MapRangeClamped` (`KismetMathLibrary.Conv_ByteToDouble` (`.B` (break `Color` (`self.Color`)))) 0.0 255.0 0.0 1.0))
  (set `self.bIsLeftSide` bIsLeftSide))

(event `self.Cube.OnClicked`
  (params (TouchedComponent :type "PrimitiveComponent Object Reference") (ButtonPressed :type "Key Structure"))
  (if (`self.bIsConnected`)
    (`/Game/AGAME/Bluerprint/Radiostation/BP_Radiostation.HandleConnectorClicked` (`self.BP_Radiostation`) self)))

(fn `UserConstructionScript`)