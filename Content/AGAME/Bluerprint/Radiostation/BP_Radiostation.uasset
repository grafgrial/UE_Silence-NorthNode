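; Radio station actor that runs a wire-matching minigame, switching the view to itself with a mouse cursor when its cube is interacted with.
; BeginPlay spawns two columns of BP_Connector actors, shuffling the colour array for each side.
; Connector clicks create a cable, attach it on an opposite-side colour match, or destroy it otherwise.
; Matches trigger a check that sets GameCompleted and prints a win message once all left connectors are connected.
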(event `self.ReceiveBeginPlay`
  (`self.SpawLeftConnectors`)
  (`self.SpawnRightConnectors`))

(event `/Game/AGAME/Base/Interface/BPI_Interaction.BPI_Iteraction`
  (params (Pawn :type "Pawn Object Reference") (Component :type "PrimitiveComponent Object Reference"))
  (bind _returnvalue (`GameplayStatics.GetPlayerController` 0))
  (if (== Component (`self.Cube`))
    (`PlayerController.SetViewTargetWithBlend` _returnvalue self 0.5 "VTBlend_Linear" 0.0 false)
    (set `PlayerController.bShowMouseCursor` true _returnvalue)
    (`self.DisableInput` Pawn _returnvalue)))

(event `SpawLeftConnectors`
  (`self.SpawConnect` (`self.LeftConnectors`) (`self.SceneLeft`) true))

(event `SpawnRightConnectors`
  (`self.SpawConnect` (`self.RightConnectors`) (`self.SceneRight`)))

(fn `CheckWinCondition`
  (params (NewParam :type "Array of /Game/AGAME/Bluerprint/Radiostation/BP_Connector Object Reference"))
  (locals (Counter :type Integer))
  (set `local.Counter` 0)
  (for _array_element NewParam
    (if (`/Game/AGAME/Bluerprint/Radiostation/BP_Connector.bIsConnected` _array_element)
      (`/Engine/EditorBlueprintResources/StandardMacros.IncrementInt` (`local.Counter`))))
  (if (== (`local.Counter`) (`KismetArrayLibrary.Array_Length` NewParam))
    (`KismetSystemLibrary.PrintString` "WIN WIN" true true (struct :`R` 0.691208 :`G` 0.102654 :`B` 1.0 :`A` 1.0) 10.0)
    (set `self.bGameCompleted` true)))

(fn `CompleteConnection`
  (params (ConnectorA :type "/Game/AGAME/Bluerprint/Radiostation/BP_Connector Object Reference") (ConnectorB :type "/Game/AGAME/Bluerprint/Radiostation/BP_Connector Object Reference"))
  (bind _currentcable (`self.CurrentCable`)
    (:`then`
      (`CableComponent.SetAttachEndTo` _currentcable ConnectorB "None" "None")
      (set `/Game/AGAME/Bluerprint/Radiostation/BP_Connector.CableReference` (`self.CurrentCable`) (`local.ConnectorA`))
      (set `/Game/AGAME/Bluerprint/Radiostation/BP_Connector.CableReference` (`self.CurrentCable`) (`local.ConnectorB`))
      (set `self.CurrentSelectedConnector` null)
      (set `self.CurrentCable` null))
    (:`else`)))

(fn `CreateAndAttachCable`
  (params (StartConnection :type "/Game/AGAME/Bluerprint/Radiostation/BP_Connector Object Reference"))
  (locals (Cable :type "CableComponent Object Reference"))
  (bind (_locationx _locationy) (`PlayerController.GetMousePosition` (`GameplayStatics.GetPlayerController` 0)))
  (bind _returnvalue (`AddComponent|NODE_AddCableComponent-1` :`RelativeTransform` (`KismetMathLibrary.MakeTransform` (`self.K2_GetActorLocation` StartConnection))))
  (bind _output_get (set `local.Cable` _returnvalue))
  (set `CableComponent.EndLocation` (`KismetMathLibrary.MakeVector` _locationx _locationy) _output_get))

(fn `DestroyCurrentCable`)

(fn `HandleConnectorClicked`
  (params (Connector :type "/Game/AGAME/Bluerprint/Radiostation/BP_Connector Object Reference"))
  (locals (ClickedConnector :type "/Game/AGAME/Bluerprint/Radiostation/BP_Connector Object Reference"))
  (bind _currentselectedconnector (`self.CurrentSelectedConnector`))
  (bind _clickedconnector (`local.ClickedConnector`))
  (bind _clickedconnector_2 (`local.ClickedConnector`))
  (bind (_color_b _color_g _color_r) (break `Color` (`/Game/AGAME/Bluerprint/Radiostation/BP_Connector.Color` (`self.CurrentSelectedConnector`))))
  (bind (_color_b_2 _color_g_2 _color_r_2) (break `Color` (`/Game/AGAME/Bluerprint/Radiostation/BP_Connector.Color` (`local.ClickedConnector`))))
  (set `local.ClickedConnector` Connector)
  (if (`self.bGameCompleted`)
    _
    (elif (== (`self.CurrentSelectedConnector`) null)
      (set `self.CurrentSelectedConnector` _clickedconnector_2)
      (bind _returnvalue (`AddComponent|NODE_AddCableComponent-0` :`RelativeTransform` (`KismetMathLibrary.MakeTransform` (`SceneComponent.K2_GetComponentLocation` (`/Game/AGAME/Bluerprint/Radiostation/BP_Connector.Cube` _clickedconnector_2)))))
      (set `self.CurrentCable` _returnvalue)
      (elif (== (`/Game/AGAME/Bluerprint/Radiostation/BP_Connector.bIsLeftSide` (`self.CurrentSelectedConnector`)) (`/Game/AGAME/Bluerprint/Radiostation/BP_Connector.bIsLeftSide` _clickedconnector_2))
        (bind _currentcable (`self.CurrentCable`)
          (:`then`
            (`ActorComponent.K2_DestroyComponent` _currentcable))
          (:`else`
            _))
        (set `self.CurrentSelectedConnector` null)
        (elif (and (== _color_b_2 _color_b) (== _color_g_2 _color_g) (== _color_r_2 _color_r))
          (`self.CompleteConnection` _currentselectedconnector _clickedconnector)
          (set `/Game/AGAME/Bluerprint/Radiostation/BP_Connector.bIsConnected` true _currentselectedconnector)
          (set `/Game/AGAME/Bluerprint/Radiostation/BP_Connector.bIsConnected` true _clickedconnector)
          (set `/Game/AGAME/Bluerprint/Radiostation/BP_Connector.ConnectedTo` (`local.ClickedConnector`) _currentselectedconnector)
          (set `/Game/AGAME/Bluerprint/Radiostation/BP_Connector.ConnectedTo` (`self.CurrentSelectedConnector`) _clickedconnector)
          (`self.CheckWinCondition` (`self.LeftConnectors`))
          (else
            (`GameplayStatics.PlaySoundAtLocation` (`self.WireSound`) (`self.K2_GetActorLocation`) (struct) 1.0 1.0 0.0 null null null)
            (bind _currentcable_2 (`self.CurrentCable`)
              (:`then`
                (`ActorComponent.K2_DestroyComponent` _currentcable_2))
              (:`else`
                _))
            (set `self.CurrentSelectedConnector` null)))))))

(fn `SpawConnect`
  (params (TargetArray :type "Array of /Game/AGAME/Bluerprint/Radiostation/BP_Connector Object Reference (by ref)") (self2 :type "SceneComponent Object Reference") (bIsLeftSide :type Boolean))
  (bind (_returnvalue_x _returnvalue_y _returnvalue_z) (`KismetMathLibrary.BreakVector` (`SceneComponent.K2_GetComponentLocation` self2)))
  (`KismetArrayLibrary.Array_Shuffle` (`self.ColorsArray`))
  (for _index (range 1 (+ (`self.ConnectorCount`) 1))
    (bind _returnvalue (`|SpawnActorFromClass` "/Game/AGAME/Bluerprint/Radiostation/BP_Connector.BP_Connector_C" (`KismetMathLibrary.MakeTransform` (`KismetMathLibrary.MakeVector` _returnvalue_x _returnvalue_y (- _returnvalue_z (* _index 10.0)))) "Undefined" "OverrideRootScale" null self null))
    (`/Game/AGAME/Bluerprint/Radiostation/BP_Connector.SpawnCon` _returnvalue (`|GetArrayItem` (`self.ColorsArray`) _index) bIsLeftSide)
    (`KismetArrayLibrary.Array_Add` TargetArray _returnvalue))
  (return))

(fn `UserConstructionScript`)