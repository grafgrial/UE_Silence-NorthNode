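; AC_Seif is an interactable actor, apparently a safe, with a hinged part that swings open and closed.
; The interaction interface event responds only to Cube5, then runs a timeline that lerps the Scene component's relative rotation between closed and 80 degrees.
; The Open flag picks the direction and flips on finish.
; A DoOnce gate, reset after each swing, blocks retriggering mid-animation.
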(event `/Game/AGAME/Base/Interface/BPI_Interaction.BPI_Iteraction`
  (params (Pawn :type "Pawn Object Reference") (Component :type "PrimitiveComponent Object Reference"))
  (bind _bopen (`self.bOpen`))
  (if (== Component (`self.Cube5`))
    (`/Engine/EditorBlueprintResources/StandardMacros.DoOnce` false :!label _label
      (:`Completed`
        (bind (_direction _alpha) (`Timeline|Timeline_0` :!via `PlayFromStart`)
          (:`Update`
            (`SceneComponent.K2_SetRelativeRotation` (`self.Scene`) (`KismetMathLibrary.RLerp` (select `bool` _bopen :`true` (struct :`Roll` 80.0) :!type "Rotator Structure") (select `bool` _bopen :`false` (struct :`Roll` 80.0) :!type "Rotator Structure") _alpha) false false))
          (:`Finished`
            (if (`self.bOpen`)
              (set `self.bOpen` false)
              (else
                (set `self.bOpen` true)))
            (`self.E_Reset`)))))))

(event `E_Reset`
  (goto _label :!via `Reset`))

(fn `UserConstructionScript`)