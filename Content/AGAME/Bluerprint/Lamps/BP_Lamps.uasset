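; Lamp actor that flickers its cube's emissive material.
; On BeginPlay a timeline track event sets Emissive to a random value, and the timeline replays five seconds after each finish.
; The same event sets PointLight intensity from an FInterpTo with no current or target input, so it resolves to zero.
; Timer, custom-event and mapped-intensity variants remain disconnected.
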(event `CustomEvent_1`)

(event `CustomEvent_0`
  (if (not (`self.Condition`))
    (`LightComponent.SetIntensity` (`self.PointLight`) 6500.0)
    (`MeshComponent.SetScalarParameterValueOnMaterials` (`self.Cube`) "Emissive" 0.6)))

(event `self.ReceiveBeginPlay`
  (`Timeline|Timeline_0` :!via `PlayFromStart` :!label _label
    (:`Finished`
      (`KismetSystemLibrary.Delay` 5.0)
      (`TimelineComponent.SetNewTime` (`self.Timeline_0`) 0.0)
      (goto _label :!via `PlayFromStart`))
    (:`NewTrack_1`
      (set `self.PARAMETR` (`KismetMathLibrary.RandomFloatInRange` 0.1 1.0))
      (`LightComponent.SetIntensity` (`self.PointLight`) (`KismetMathLibrary.FInterpTo` 0.0 0.0 (`GameplayStatics.GetWorldDeltaSeconds`) 2.0))
      (`MeshComponent.SetScalarParameterValueOnMaterials` (`self.Cube`) "Emissive" (`self.PARAMETR`)))))

(fn `UserConstructionScript`)