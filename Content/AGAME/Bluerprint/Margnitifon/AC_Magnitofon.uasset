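; Interactable tape recorder actor that toggles music playback when a player interacts with its mesh.
; Starting copies music and duration arrays from the DA list, using a separate random index for each.
; It blocking-loads a random track, plays it, waits its listed duration, removes it and calls Restart for the next.
; Sphere overlap checks trigger nothing, and the widget-opening code is unconnected.
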(event `self.Sphere.OnComponentBeginOverlap`
  (params (OverlappedComponent :type "PrimitiveComponent Object Reference") (OtherActor :type "Actor Object Reference") (OtherComp :type "PrimitiveComponent Object Reference") (OtherBodyIndex :type Integer) (bFromSweep :type Boolean) (SweepResult :type "HitResult Structure (by ref)"))
  (if (`KismetSystemLibrary.DoesImplementInterface` OtherActor "/Game/AGAME/Base/Interface/BPI_PLayer.BPI_Player_C")
    _))

(event `self.Sphere.OnComponentEndOverlap`
  (params (OverlappedComponent :type "PrimitiveComponent Object Reference") (OtherActor :type "Actor Object Reference") (OtherComp :type "PrimitiveComponent Object Reference") (OtherBodyIndex :type Integer))
  (if (`KismetSystemLibrary.DoesImplementInterface` OtherActor "/Game/AGAME/Base/Interface/BPI_PLayer.BPI_Player_C")
    _))

(event `/Game/AGAME/Base/Interface/BPI_Interaction.BPI_Iteraction`
  (params (Pawn :type "Pawn Object Reference") (Component :type "PrimitiveComponent Object Reference"))
  (if (== Component (`self.Mesh`))
    (`self.E_play`)))

(event `Restart`
  (bind _audio (`self.Audio`))
  ;[1 1 1] Comment
  (if (not (`AudioComponent.IsPlaying` (`self.Audio`)))
    (set `self.Index` (`KismetMathLibrary.RandomIntegerInRange` 0 (`KismetArrayLibrary.Array_LastIndex` (`self.STR Music`))) :!label _label)
    (bind _returnvalue (`KismetSystemLibrary.LoadAsset_Blocking` (`|GetArrayItem` (`self.STR Music`) (`self.Index`))))
    (bind _assound_base (cast `SoundBase` _returnvalue))
    (`AudioComponent.SetSound` _audio _assound_base)
    (`AudioComponent.Play` _audio 0.0)
    (`KismetSystemLibrary.Delay` (+ (`|GetArrayItem` (`self.STR Time`) (`self.Index`)) 0.4))
    (`KismetArrayLibrary.Array_Remove` (`self.STR Music`) (`self.Index`))
    (`KismetArrayLibrary.Array_Remove` (`self.STR Time`) (`self.Index`))
    (`KismetSystemLibrary.Delay` 0.3)
    (`self.Restart`)))

(event `E_play`
  (bind _da (`self.DA`))
  (bind (_str_music _str_time) (break `/Game/AGAME/Bluerprint/Margnitifon/DataAssets/STR_Magnitofon` (`/Game/AGAME/Bluerprint/Margnitifon/DataAssets/PDA_Magnitofon.STR` (`|GetArrayItem` _da (`KismetMathLibrary.RandomIntegerInRange` 0 (`KismetArrayLibrary.Array_LastIndex` _da))))))
  (if (`self.Is Play`)
    (`AudioComponent.Stop` (`self.Audio`))
    (set `self.Is Play` false)
    (else
      (set `self.Is Play` true)
      (set `self.STR Music` _str_music)
      (set `self.STR Time` _str_time)
      (goto _label))))

(fn `BPI_LookAt`
  (returns (Message :type Text))
  (return ""))

(fn `UserConstructionScript`
  (`SphereComponent.SetSphereRadius` (`self.Sphere`) (`self.In Sphere Radius`) true))